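; BP_Aircraft is an aircraft actor that drops bombs on input and prints debug readouts.
; The IA_FireBomb input spawns a BP_Bomb at the Bombpoint component's world transform.
; Tick prints truncated game time and the distance between the stored Distance vector and the actor's location, converted to a vector and truncated.
; Both prints share one key, and Tick only reassigns Distance to itself.
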(event `self.ReceiveTick`
  (params (DeltaSeconds :type "Float (single-precision)"))
  (set `self.distance` (`self.distance`))
  (`KismetSystemLibrary.PrintString` (`KismetStringLibrary.Conv_IntToString` (`KismetMathLibrary.FTrunc` (`GameplayStatics.GetTimeSeconds`))) true true (struct :`G` 0.66 :`B` 1.0 :`A` 1.0) 0.01 "1")
  (`KismetSystemLibrary.PrintString` (`KismetStringLibrary.Conv_IntVectorToString` (`KismetMathLibrary.FTruncVector` (`KismetMathLibrary.Conv_DoubleToVector` (`KismetMathLibrary.Vector_Distance` (`self.distance`) (`self.K2_GetActorLocation`))))) true true (struct :`G` 0.66 :`B` 1.0 :`A` 1.0) 0.01 "1"))

(event `EnhancedInput|/Game/LEC10/IA_FireBomb`
  (params (ActionValue :type Boolean) (ElapsedSeconds :type "Float (double-precision)") (TriggeredSeconds :type "Float (double-precision)") (InputAction :type "InputAction Object Reference" :default "/Game/LEC10/IA_FireBomb.IA_FireBomb"))
  (:`Started`
    (`|SpawnActorFromClass` "/Game/LEC10/BP_Bomb.BP_Bomb_C" (`SceneComponent.K2_GetComponentToWorld` (`self.bombpoint`)) "Undefined" "MultiplyWithRoot" null null)))

(fn `UserConstructionScript`)